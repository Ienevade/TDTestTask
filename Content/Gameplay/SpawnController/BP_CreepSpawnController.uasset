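; Creep wave spawn controller that sequences waves, groups and creep subgroups from three hard-coded DT_Waves rows loaded on BeginPlay.
; Tick counts down SpawnTimer and steps a flag-and-index state machine, firing wave events, with automatic or manual (StartNextWave) starts.
; SpawnCreep is a stub that only prints the creep name.
; InitCampaign, StartWave and SpawnGroup form a separate timer-based sequence that the Tick path never calls.
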(event EventTick
  (params (DeltaSeconds :type Float%20%28single-precision%29))
  (CallFunction|UpdateTimer DeltaSeconds)
  (CallFunction|UpdateSpawn))

(event EventBeginPlay
  (CallFunction|InitSpawnData))

(fn ConstructionScript)

(fn InitCampaign
  (bind _waves (Variables|Default|GetWaves))
  (bind _output (Utilities|Array|Get(acopy) _waves))
  (bind _wavedelay (Utilities|Struct|BreakS_Wave _output))
  (bind _returnvalue (Math|Float|Clamp(Float) _wavedelay 0.1 1e+03))
  (for _array_element (Utilities|Array|MakeArray "L1W1" "L1W2" "L1W3")
    (bind _returnvalue_2 (Utilities|GetDataTableRow "/Game/Data/DT_Waves.DT_Waves" _array_element)
      (:then
        (Utilities|Array|Add (Variables|Default|GetWaves) _returnvalue_2))))
  (bind _returnvalue_3 (Utilities|Time|SetTimerbyEvent (EventDispatchers|CreateEvent :!event StartWave) _returnvalue))
  (bind _output_get (Variables|Default|SetWaveTimer _returnvalue_3))
  (Default|CallWaveTimerStarted _output_get _returnvalue self))

(fn StartWave
  (bind _waves (Variables|Default|GetWaves))
  (bind _currentwave (Variables|Default|GetCurrentWave))
  (bind _waves_2 (Variables|Default|GetWaves))
  (bind _currentwave_2 (Variables|Default|GetCurrentWave))
  (bind _currentwave_3 (Variables|Default|GetCurrentWave))
  (bind _output (Utilities|Array|Get(acopy) _waves _currentwave))
  (bind _output_2 (Utilities|Array|Get(acopy) _waves_2 _currentwave_2))
  (bind _groups (Utilities|Struct|BreakS_Wave _output_2))
  (bind _wavedelay (Utilities|Struct|BreakS_Wave _output))
  (bind _returnvalue (Math|Float|Clamp(Float) _wavedelay 0.1 1e+03))
  (Default|CallOnWaveStarted self)
  (if (> (Utilities|Array|Length _groups) (Variables|Default|GetCurrentGroup))
    (if (.SpawnOnLastGroupDead (Utilities|Struct|BreakS_Group (Utilities|Array|Get(acopy) _groups (Variables|Default|GetCurrentGroup))))
      _
      (else
        _))
    (bind _returnvalue_2 (Utilities|Time|SetTimerbyEvent (EventDispatchers|CreateEvent :!event SpawnGroup) (Math|Float|Clamp(Float) (.SpawnDelay (Utilities|Struct|BreakS_Group (Utilities|Array|Get(acopy) _groups (Variables|Default|GetCurrentGroup)))) 0.1 1e+03)))
    (Variables|Default|SetGroupTimer _returnvalue_2)
    (else
      (Math|Integer|IncrementInt _currentwave_3
        (:%20%20
          (if (> (Utilities|Array|Length (Variables|Default|GetWaves)) _currentwave_3)
            (Variables|Default|SetCurrentGroup 0)
            (Variables|Default|SetCurrentCreepType 0)
            (Variables|Default|SetCurrentCreep 0)
            (Default|CallOnWaveEnd self)
            (if (Variables|Default|GetAutoStartNextWave)
              (bind _returnvalue_3 (Utilities|Time|SetTimerbyEvent (EventDispatchers|CreateEvent :!event StartWave) _returnvalue))
              (bind _output_get (Variables|Default|SetWaveTimer _returnvalue_3))
              (Default|CallWaveTimerStarted _output_get _returnvalue self)
              (Variables|Default|SetIfWaveTimerStarted true)
              (else
                (Variables|Default|SetIfWaveTimerStarted false)))
            (else
              (Default|CallOnWavesEnded self))))))))

(fn SpawnGroup
  (bind _waves (Variables|Default|GetWaves))
  (bind _currentwave (Variables|Default|GetCurrentWave))
  (bind _currentgroup (Variables|Default|GetCurrentGroup))
  (bind _output (Utilities|Array|Get(acopy) _waves _currentwave))
  (bind (_wavedelay _creeps _groups) (Utilities|Struct|BreakS_Wave _output))
  (bind _output_2 (Utilities|Array|Get(acopy) _groups _currentgroup))
  (bind (_spawnonlastgroupdead _spawndelay _creeps_2) (Utilities|Struct|BreakS_Group _output_2))
  (if (> (Utilities|Array|Length _creeps_2) (Variables|Default|GetCurrentCreepType))
    (Development|PrintString (Utilities|String|Append "CreepSpawned: " (Utilities|String|ToString(Name) (.CreepName (Utilities|Struct|BreakS_GroupCreep (Utilities|Array|Get(acopy) _creeps (.Creep (Utilities|Struct|BreakS_CreepCount (Utilities|Array|Get(acopy) _creeps_2 (Variables|Default|GetCurrentCreepType))))))))))
    (bind _result (Math|Integer|IncrementInt (Variables|Default|GetCurrentCreep))
      (:%20%20
        (if (>= _result (.Count (Utilities|Struct|BreakS_CreepCount (Utilities|Array|Get(acopy) _creeps_2 (Variables|Default|GetCurrentCreepType)))))
          (Math|Integer|IncrementInt (Variables|Default|GetCurrentCreepType)
            (:%20%20
              (Variables|Default|SetCurrentCreep 0))))
        (bind _returnvalue (Utilities|Time|SetTimerbyEvent (EventDispatchers|CreateEvent :!event SpawnGroup) (Math|Float|Clamp(Float) _spawndelay 0.01 1e+04)))
        (Variables|Default|SetGroupDelayTimer _returnvalue)))
    (else
      (Variables|Default|SetCurrentCreepType 0)
      (Math|Integer|IncrementInt (Variables|Default|GetCurrentGroup)
        (:%20%20
          (CallFunction|StartWave))))))

(fn ResetController
  (Variables|Default|SetScenarioEnded false)
  (Variables|Default|SetFirstCreepSpawned false)
  (Variables|Default|SetWaveStarted false)
  (Variables|Default|SetCurrentWave -1)
  (Variables|Default|SetCurrentGroup 0)
  (Variables|Default|SetCurrentCreepType 0)
  (Variables|Default|SetCurrentCreep 0)
  (Variables|Default|SetCurrentSubGroup 0)
  (Utilities|Array|Clear (Variables|Default|GetWaves))
  (Utilities|Time|ClearandInvalidateTimerbyHandle (Variables|Default|GetWaveTimer))
  (Utilities|Time|ClearandInvalidateTimerbyHandle (Variables|Default|GetGroupTimer))
  (Utilities|Time|ClearandInvalidateTimerbyHandle (Variables|Default|GetGroupDelayTimer))
  (Variables|Default|SetFirstCreepSpawned false)
  (CallFunction|SpawnCreep "base" 1e+02 0.0 true))

(fn InitCampaignbyName
  (params (CampaignName :type Name))
  (bind _waves (Variables|Default|GetWaves))
  (bind _currentwave (Variables|Default|GetCurrentWave))
  (bind _output (Utilities|Array|Get(acopy) _waves _currentwave))
  (bind _wavedelay (Utilities|Struct|BreakS_Wave _output))
  (bind _returnvalue (Math|Float|Clamp(Float) _wavedelay 0.1 1e+03))
  (for _array_element (Utilities|Array|MakeArray "L1W1" "L1W2" "L1W3")
    (bind _returnvalue_2 (Utilities|GetDataTableRow "/Game/Data/DT_Waves.DT_Waves" _array_element)
      (:then
        (Utilities|Array|Add (Variables|Default|GetWaves) _returnvalue_2))))
  (bind _returnvalue_3 (Utilities|Time|SetTimerbyEvent (EventDispatchers|CreateEvent :!event StartWave) _returnvalue))
  (bind _output_get (Variables|Default|SetWaveTimer _returnvalue_3))
  (Default|CallWaveTimerStarted _output_get _returnvalue self)
  (Variables|Default|SetIfWaveTimerStarted true))

(fn StartNextWave
  (bind _self self)
  (if (not (Variables|Default|GetStartWaveAuto))
    (if (not (Variables|Default|GetWaveStarted))
      (if (> (Utilities|Array|Length (Variables|Default|GetWaves)) (Variables|Default|GetCurrentWave))
        (Math|Integer|IncrementInt (Variables|Default|GetCurrentWave)
          (:%20%20
            (bind _output_get (Variables|Default|SetSpawnTimer (Utilities|Struct|BreakS_Wave (Utilities|CurrWave))))
            (Variables|Default|SetWaveStarted true)
            (Default|CallWaveTimerStarted :Time _output_get :Controller _self)
            (Default|CallOnWaveStarted _self)))
        (else
          (Variables|Default|SetScenarioEnded true)
          (Default|CallOnWavesEnded self))))))

(fn UpdateSpawn
  (bind _output (Utilities|CurrCreepInfo))
  (if (<= (Variables|Default|GetSpawnTimer) 0.0)
    (if (Variables|Default|GetWaveStarted)
      (if (and (.SpawnOnLastGroupDead (Utilities|Struct|BreakS_Group (Utilities|CurrGroup))) (not (Variables|Default|GetGroupStarted)))
        _
        (else
          _))
      (if (Variables|Default|GetGroupStarted)
        (if (> (Utilities|Array|Length (Utilities|Struct|BreakS_Group (Utilities|CurrGroup))) (Variables|Default|GetCurrentSubGroup))
          (if (> (.count (Utilities|CurrSubGroup)) (Variables|Default|GetCurrentCreep))
            (Variables|Default|SetSpawnTimer (Utilities|Struct|BreakS_Group (Utilities|CurrGroup)))
            (CallFunction|SpawnCreep (.creepname _output) (.hp _output) (.reward _output) false)
            (Variables|Default|SetFirstCreepSpawned true)
            (Math|Integer|IncrementInt (Variables|Default|GetCurrentCreep))
            (else
              (Math|Integer|IncrementInt (Variables|Default|GetCurrentSubGroup))))
          (else
            (Variables|Default|SetGroupStarted false)
            (Math|Integer|IncrementInt (Variables|Default|GetCurrentGroup)
              (:%20%20
                (Variables|Default|SetCurrentSubGroup 0)))))
        (elif (> (Utilities|Array|Length (Utilities|Struct|BreakS_Wave (Utilities|CurrWave))) (Variables|Default|GetCurrentGroup))
          (Variables|Default|SetGroupStarted true)
          (else
            (Variables|Default|SetWaveStarted false)
            (Variables|Default|SetCurrentGroup 0)
            (Default|CallOnWaveEnd self)
            (if (Variables|Default|GetAutoStartNextWave)
              (Math|Integer|IncrementInt (Variables|Default|GetCurrentWave))
              (elif (not (> (Utilities|Array|Length (Variables|Default|GetWaves)) (Variables|Default|GetCurrentWave)))
                (Variables|Default|SetScenarioEnded true)
                (Default|CallOnWavesEnded self))))))
      (elif (Variables|Default|GetStartWaveAuto)
        (if (> (- (Utilities|Array|Length (Variables|Default|GetWaves)) 1) (Variables|Default|GetCurrentWave))
          (Variables|Default|SetSpawnTimer (Utilities|Struct|BreakS_Wave (Utilities|CurrWave)))
          (Variables|Default|SetWaveStarted true)
          (else
            (Variables|Default|SetScenarioEnded true)
            (Default|CallOnWavesEnded self)))))))

(fn SpawnCreep
  (params (Name :type Name) (CreepHP :type Float%20%28single-precision%29) (CreepReward :type Float%20%28single-precision%29) (Base :type Boolean))
  (Development|PrintString (Utilities|String|Append "CreepSpawned: " (Utilities|String|ToString(Name) Name)) true true "(R=0.000000,G=0.660000,B=1.000000,A=1.000000)" 1e+02))

(fn UpdateTimer
  (params (SecDelta :type Float%20%28single-precision%29))
  (if (> (Variables|Default|GetSpawnTimer) 0.0)
    (Variables|Default|SetSpawnTimer (- (Variables|Default|GetSpawnTimer) SecDelta))))

(fn InitSpawnData
  (Utilities|Array|Clear (Variables|Default|GetWaves))
  (for _array_element (Utilities|Array|MakeArray "L1W1" "L1W2" "L1W3")
    (bind _returnvalue (Utilities|GetDataTableRow "/Game/Data/DT_Waves.DT_Waves" _array_element)
      (:then
        (Utilities|Array|Add (Variables|Default|GetWaves) _returnvalue)))))

(fn InitController
  (params (CampaignName :type Name))
  (Variables|Default|SetCampaignName CampaignName))